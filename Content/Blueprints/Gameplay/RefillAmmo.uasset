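; Ammo refill station that refills a Character_Gameplay's ammo on sphere overlap, then locks itself for a cooldown.
; A pickup calls PickUpAmmo, plays a sound, swaps the sphere to its unusable material and toggles a countdown text.
; A looping one-second timer decrements the countdown until it reaches MinTime, then clears itself, re-enables refilling, restores the usable material and toggles the text again.
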(event OnComponentBeginOverlap(Sphere)
  (params (OverlappedComponent :type Primitive%20Component%20Object%20Reference) (OtherActor :type Actor%20Object%20Reference) (OtherComp :type Primitive%20Component%20Object%20Reference) (OtherBodyIndex :type Integer) (bFromSweep :type Boolean) (SweepResult :type Hit%20Result%20Structure%20%28by%20ref%29))
  (if (Variables|Default|GetCanRefill?)
    (bind _ascharacter_gameplay (Utilities|Casting|CastToCharacter_Gameplay OtherActor))
    (Default|PickUpAmmo _ascharacter_gameplay)
    (CallFunction|PlayerAmmoRefilled)
    (CallFunction|StartTimer)))

(event Custom|StartTimer
  (bind _returnvalue (Utilities|Time|SetTimerbyEvent (delegate Custom|CoolDownTimer) 1.0 true)))

(event Custom|CoolDownTimer
  (if (not (== (Variables|Default|GetCountDownTime) (Variables|Default|GetMinTime)))
    (CallFunction|TimerIsRunning)
    (else
      (Utilities|Time|ClearandInvalidateTimerbyHandle (stale Custom|StartTimer _returnvalue))
      (Variables|Default|SetCanRefill? true)
      (Rendering|Material|SetMaterial (Variables|Default|GetSphere1) 0 (Variables|Default|GetCanBeUsedMaterial))
      (Rendering|ToggleVisibility (Variables|Default|GetTextRender) false))))

(event Custom|TimerIsRunning
  (CallFunction|Countdown)
  (Variables|Default|SetCanRefill? false))

(event Custom|PlayerAmmoRefilled
  (Variables|Default|SetCountDownTime (Variables|Default|GetMaxTime))
  (Variables|Default|SetCanRefill? false)
  (Audio|SpawnSoundatLocation 0 (Transformation|GetActorLocation) "0, 0, 0" 1.0 1.0 0.0 0 0)
  (Rendering|Components|TextRender|SetText (Variables|Default|GetTextRender) (Utilities|Text|ToText(Integer) (Variables|Default|GetCountDownTime)))
  (Rendering|ToggleVisibility (Variables|Default|GetTextRender) true)
  (Rendering|Material|SetMaterial (Variables|Default|GetSphere1) 0 (Variables|Default|GetCantBeUsedMaterial)))

(fn ConstructionScript)

(fn Countdown
  (bind _result (Math|Integer|DecrementInt (Variables|Default|GetCountDownTime))
    (:%20%20
      (Rendering|Components|TextRender|SetText (Variables|Default|GetTextRender) (Utilities|Text|ToText(Integer) _result)))))