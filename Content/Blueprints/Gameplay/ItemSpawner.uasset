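; ItemSpawner spawns Item_Base actors at its Arrow component's location, provided the spawn area is not blocked by another item.
; Box overlap events clear CanSpawnItem when an Item_Base enters and set it again when any Item_Base leaves, without counting remaining overlaps.
; SpawnItem checks that flag before spawning and has no caller within this Blueprint.
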(event OnComponentBeginOverlap(Box)
  (params (OverlappedComponent :type Primitive%20Component%20Object%20Reference) (OtherActor :type Actor%20Object%20Reference) (OtherComp :type Primitive%20Component%20Object%20Reference) (OtherBodyIndex :type Integer) (bFromSweep :type Boolean) (SweepResult :type Hit%20Result%20Structure%20%28by%20ref%29))
  (Utilities|Casting|CastToItem_Base OtherActor)
  (Variables|Default|SetCanSpawnItem? false))

(event OnComponentEndOverlap(Box)
  (params (OverlappedComponent :type Primitive%20Component%20Object%20Reference) (OtherActor :type Actor%20Object%20Reference) (OtherComp :type Primitive%20Component%20Object%20Reference) (OtherBodyIndex :type Integer))
  (Utilities|Casting|CastToItem_Base OtherActor)
  (Variables|Default|SetCanSpawnItem? true))

(fn ConstructionScript)

(fn SpawnItem
  (if (Variables|Default|GetCanSpawnItem?)
    (Game|SpawnActorfromClass :Class "/Game/Blueprints/Gameplay/Item_Base.Item_Base_C" :SpawnTransform (Math|Transform|MakeTransform (Transformation|GetWorldLocation (Variables|Default|GetArrow)) "0, 0, 0" "1.000000,1.000000,1.000000") :CollisionHandlingOverride "Undefined" :TransformScaleMethod "MultiplyWithRoot" :ItemEnumArray "NewEnumerator28" :Instigator 0)))