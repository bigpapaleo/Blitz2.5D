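; Team-colored ball projectile that refills a teammate's ball count or freezes an opposing player on overlap, then destroys itself.
; BeginPlay briefly disables sphere collision to avoid sticking to the player and sets the material from the current team.
; After a decay delay, a timeline pulses the material's glow, and its first update starts the delay that destroys the ball.
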(event OnComponentBeginOverlap(CollisionSphere)
  (params (OverlappedComponent :type Primitive%20Component%20Object%20Reference) (OtherActor :type Actor%20Object%20Reference) (OtherComp :type Primitive%20Component%20Object%20Reference) (OtherBodyIndex :type Integer) (bFromSweep :type Boolean) (SweepResult :type Hit%20Result%20Structure%20%28by%20ref%29))
  (Development|PrintString (Utilities|GetDisplayName OtherActor))
  (bind _ascharacter_gameplay (Utilities|Casting|CastToCharacter_Gameplay OtherActor))
  (if (Utilities|Enum|Equal(Enum) (Variables|Default|GetCurrent%20Team) (Variables|/Game/Blueprints/Gameplay/Character_Gameplay.Character_Gameplay_C|GetTeam _ascharacter_gameplay))
    (Default|IncreaseBallCount _ascharacter_gameplay)
    (Actor|DestroyActor)
    (else
      (Default|PlayerIsFrozen _ascharacter_gameplay)
      (Actor|DestroyActor))))

(event Custom|BallDeathTimer_MC
  (Utilities|FlowControl|Delay (Variables|Default|GetTimeBeforeDecayStarts))
  ;[0.15 0 0.04405 0.5] NEEDS TO GLOW!
  (bind _pulse (Timeline|TimelineGlow PlayFromStart)
    (:Update
      (Rendering|Material|SetScalarParameterValueonMaterials (Variables|Default|GetSphere) "Pulse" _pulse)
      (Utilities|FlowControl|Delay (Variables|Default|GetDeathTimeOfBall))
      (Actor|DestroyActor))))

(event EventBeginPlay
  (Utilities|FlowControl|Sequence
    (:then_0
      ;[0.15 0.15 0.15 0.5] This stops the ball getting stuck on player
      (Collision|SetCollisionEnabled (Variables|Default|GetCollisionSphere) "NoCollision")
      (Utilities|FlowControl|Delay 0.001)
      (Collision|SetCollisionEnabled (Variables|Default|GetCollisionSphere) "QueryAndProbe"))
    (:then_1
      ;[0.15 0.15 0.15 0.5] Set up team info
      (CallFunction|PickTeamColor (Variables|Default|GetCurrent%20Team)))
    (:then_2
      (Utilities|FlowControl|Delay (Variables|Default|GetTimeBeforeDecayStarts))
      ;[0.15 0 0.04405 0.5] NEEDS TO GLOW!
      (bind _pulse (Timeline|TimelineGlow PlayFromStart)
        (:Update
          (Rendering|Material|SetScalarParameterValueonMaterials (Variables|Default|GetSphere) "Pulse" _pulse)
          (Utilities|FlowControl|Delay (Variables|Default|GetDeathTimeOfBall))
          (Actor|DestroyActor))))))

(fn ConstructionScript)

(fn PickTeamColor
  (params (Team :type AssignTeam_Enum%20Enum :default "NewEnumerator0"))
  (Rendering|Material|SetMaterial (Variables|Default|GetSphere) 0 (Utilities|Select :Index Team :NewEnumerator0 "/Game/Art/Team1BallBaseMaterail_Inst1.Team1BallBaseMaterail_Inst1" :NewEnumerator1 "/Game/Art/Team2.Team2")))

(fn OnRepTimeBeforeDecayStarts)

(fn OnRepDeathTimeOfBall)