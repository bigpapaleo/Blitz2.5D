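; Game mode for local multiplayer that spawns up to two players and starts the shared gameplay camera on BeginPlay.
; It caches all PlayerStarts, then matches their tags to each player index up to PlayerCount, a zero-based count set by the Start_Menu widget.
; Each match creates a local player and possesses a spawned Character_Gameplay, with the second assigned another team.
; Finally it triggers GoFromGameMode on every Camera_GamePlayLocal actor.
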(event EventBeginPlay
  (|CallParentFunction)
  (CallFunction|GetPlayerStarts)
  (CallFunction|SpawnPlayers)
  (CallFunction|SetUpCamera))

(event EventTick
  (params (DeltaSeconds :type Float%20%28single-precision%29))
  (|CallParentFunction DeltaSeconds) ; This node is disabled and will not be called.\nDrag off pins to build functionality.
)

(fn ConstructionScript
  (|CallParentFunction))

(fn SpawnPlayers
  ;[1 1 1] Number of players (Zero-based numbering) This is set in Start_Menu widget
  (for _index (range 0 (Variables|Default|GetPlayerCount))
    (for _array_element (Variables|Default|GetPlayerStartArray)
      (if (Utilities|Name|Equal(Name) (Variables|/Script/Engine.PlayerStart|GetPlayerStartTag _array_element) (Utilities|String|StringToName (Utilities|String|ToString(Integer) _index)))
        (switch int _index
          (:0
            (Class|GameplayStatics|CreatePlayer 0)
            (bind _returnvalue (Game|SpawnActorfromClass "/Game/Blueprints/Gameplay/Character_Gameplay.Character_Gameplay_C" (Transformation|GetActorTransform _array_element) "Undefined" "MultiplyWithRoot" 0 "NewEnumerator0" 0))
            (Pawn|Possess (Game|GetPlayerController 0) _returnvalue))
          (:1
            (Class|GameplayStatics|CreatePlayer 1)
            (bind _returnvalue_2 (Game|SpawnActorfromClass "/Game/Blueprints/Gameplay/Character_Gameplay.Character_Gameplay_C" (Transformation|GetActorTransform _array_element) "Undefined" "MultiplyWithRoot" 0 "NewEnumerator1" 0))
            (Pawn|Possess (Game|GetPlayerController 1) _returnvalue_2))
          (:2))))))

(fn GetPlayerStarts
  (bind _outactors (Actor|GetAllActorsOfClass "/Script/Engine.PlayerStart"))
  (Variables|Default|SetPlayerStartArray _outactors))

(fn SetUpCamera
  (bind _outactors (Actor|GetAllActorsOfClass "/Game/Blueprints/Gameplay/Camera_GamePlay-Local.Camera_GamePlay-Local_C"))
  (for _array_element _outactors
    (Default|GofromGameMode _array_element)))