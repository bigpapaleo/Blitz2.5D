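; Gameplay game mode that periodically spawns items during a match through ItemSpawner actors placed in the level.
; On BeginPlay it starts a looping timer whose interval is randomized once, within a range of up to fifteen seconds.
; Each timer tick gathers all ItemSpawner actors and calls SpawnItem on one chosen at random.
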(event Custom|SpawnAnItemFromSpawner
  (bind _outactors (Actor|GetAllActorsOfClass "/Game/Blueprints/Gameplay/ItemSpawner.ItemSpawner_C"))
  (Default|SpawnItem (.OutItem (Utilities|Array|Random _outactors))))

(event Custom|StartTimerForItemSpawner
  (Utilities|Time|SetTimerbyEvent (delegate Custom|SpawnAnItemFromSpawner) (Math|Random|RandomFloatinRange 0.0 15.0) true))

(event EventBeginPlay
  (|CallParentFunction)
  (CallFunction|StartTimerforItemSpawner))

(event EventTick
  (params (DeltaSeconds :type Float%20%28single-precision%29))
  (|CallParentFunction DeltaSeconds) ; This node is disabled and will not be called.\nDrag off pins to build functionality.
)

(fn ConstructionScript
  (|CallParentFunction))